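; BP_TrafficLightsManager drives every BP_TraffictLight in the level through one shared color sequence.
; Shortly after BeginPlay, it gathers the lights and reads the color keys from the ColorSettings map.
; A recursive ColorsIterator event applies each color's mapped value to all lights via ChangeColor, then waits a per-color delay before advancing.
; The sequence stops after the last key, with no restart.
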(event Custom|Recolor
  (Utilities|FlowControl|Delay 2.0)
  (bind _outactors (Actor|GetAllActorsOfClass "/Game/Blueprints/BP_TraffictLight.BP_TraffictLight_C"))
  (Variables|Default|SetTariffLights _outactors)
  (bind _keys (Utilities|Map|Keys (Utilities|Struct|BreakS_LIghtColor (Variables|Default|GetColorSettings))))
  (CallFunction|ColorsIterator _keys))

(event Custom|ColorsIterator
  (params (ColorArray :type Array%20of%20E_LightColor%20Enums :default "NewEnumerator0") (Index :type Integer))
  (bind _output (Utilities|Array|Get(acopy) ColorArray Index))
  (CallFunction|SetColorforAllActors _output)
  (bind _seconds (CallFunction|DelayOfLightColor _output))
  (Utilities|FlowControl|Delay _seconds)
  (bind _result (Math|Integer|IncrementInt Index)
    (:%20%20
      (if (< _result (Utilities|Array|Length ColorArray))
        (CallFunction|ColorsIterator ColorArray _result)))))

(event EventBeginPlay
  (CallFunction|Recolor))

(fn ConstructionScript)

(fn SetColorforAllActors
  (params (Color :type E_LightColor%20Enum :default "NewEnumerator0"))
  (for _array_element (Variables|Default|GetTariffLights)
    (Default|ChangeColor _array_element (.Value (Utilities|Map|Find (Utilities|Struct|BreakS_LIghtColor (Variables|Default|GetColorSettings)) Color)))))

(fn DelayOfLightColor
  (params (Color :type E_LightColor%20Enum :default "NewEnumerator0"))
  (switch Utilities|FlowControl|Switch|SwitchonE_LightColor Color
    (:NewEnumerator0
      (return 5.0))
    (:NewEnumerator1
      (return 1.0))
    (:NewEnumerator2
      (return 3.0))))